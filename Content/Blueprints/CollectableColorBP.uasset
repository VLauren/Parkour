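; Collectable color pickup for a parkour game that unlocks one of four colors when an actor overlaps it.
; On overlap, it prints the collected color, casts the game mode to ParkourGameModeBP and switches on its Color enum to set the matching active flag.
; The pickup then destroys itself, or prints a failure message if the cast fails.
; Any overlapping actor triggers it, as the other actor is never checked.
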(event EventBeginPlay)

(event Collision|EventActorBeginOverlap
  (params (OtherActor :type Actor%20Object%20Reference))
  (Development|PrintString (Utilities|String|Append "Color recogido: " (Utilities|String|EnumtoString (Variables|Default|GetColor))) true true "(R=0.000000,G=1.000000,B=0.033423,A=1.000000)")
  (bind _asparkour_game_mode_bp (Utilities|Casting|CastToParkourGameModeBP (Game|GetGameMode))
    (:then
      (switch Utilities|FlowControl|Switch|SwitchonColors (Variables|Default|GetColor)
        (:NewEnumerator0
          (Variables|/Game/Blueprints/ParkourGameModeBP.ParkourGameModeBP_C|SetColor1Active _asparkour_game_mode_bp true))
        (:NewEnumerator1
          (Variables|/Game/Blueprints/ParkourGameModeBP.ParkourGameModeBP_C|SetColor2Active _asparkour_game_mode_bp true))
        (:NewEnumerator2
          (Variables|/Game/Blueprints/ParkourGameModeBP.ParkourGameModeBP_C|SetColor3Active _asparkour_game_mode_bp true))
        (:NewEnumerator3
          (Variables|/Game/Blueprints/ParkourGameModeBP.ParkourGameModeBP_C|SetColor4Active _asparkour_game_mode_bp true)))
      (Actor|DestroyActor))
    (:CastFailed
      (Development|PrintString "CAST FAILED"))))

(event EventTick
  (params (DeltaSeconds :type Float%20%28single-precision%29)))

(fn ConstructionScript)