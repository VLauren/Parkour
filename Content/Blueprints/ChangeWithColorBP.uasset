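; ChangeWithColorBP is a component that changes its owning actor once a given color becomes active in the parkour game.
; At begin play it sets the owner's collision to the inverse of EnableColisionWithColor.
; Each tick it polls ParkourGameModeBP for ColorToCheck until that color is active.
; It then stops checking, applies MaterialToSet to the static mesh's first two slots and enables collision regardless of that flag.
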(event EventBeginPlay
  ;[0.1562 0.1562 0.1562] Colision inicial
  (Collision|SetActorEnableCollision (Components|GetOwner) (not (Variables|Default|GetEnableColisionWithColor))))

(event EventTick
  (params (DeltaSeconds :type Float%20%28single-precision%29))
  (bind _returnvalue (Components|GetOwner))
  (bind _materialtoset (Variables|Default|GetMaterialToSet))
  (bind _returnvalue_2 (Actor|GetComponentbyClass _returnvalue "/Script/Engine.StaticMeshComponent"))
  ;[0.07227 0.1302 0.07475] Comprobacion periodica
  (if (not (Variables|Default|GetStopChecking))
    (bind _asparkour_game_mode_bp (Utilities|Casting|CastToParkourGameModeBP (Game|GetGameMode)))
    (bind _isactive (Default|IsColorActive _asparkour_game_mode_bp (Variables|Default|GetColorToCheck)))
    (if _isactive
      (Variables|Default|SetStopChecking true)
      (Utilities|FlowControl|Sequence
        (:then_0
          ;[0.1562 0.1562 0.1562] Cambio de material
          (Rendering|Material|SetMaterial _returnvalue_2 0 _materialtoset)
          (Rendering|Material|SetMaterial _returnvalue_2 1 _materialtoset))
        (:then_1
          ;[0.1615 0.1615 0.1615] Cambio de colision
          (Collision|SetActorEnableCollision (Components|GetOwner) true))))))