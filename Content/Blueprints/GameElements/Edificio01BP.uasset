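; Edificio01BP is a building in a parkour game that changes materials when certain colors become active.
; Every Tick, two independent checks ask ParkourGameModeBP whether their color is active.
; When one is, it swaps its own material slot on the static mesh (index 0 or 2) and sets a stop flag so that check does not repeat.
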(event EventBeginPlay)

(event Collision|EventActorBeginOverlap
  (params (OtherActor :type Actor%20Object%20Reference)))

(event EventTick
  (params (DeltaSeconds :type Float%20%28single-precision%29))
  (Utilities|FlowControl|Sequence
    (:then_0
      ;[0.07227 0.1302 0.07475] Comprobacion periodica
      (if (not (Variables|Default|GetStopChecking1))
        (bind _asparkour_game_mode_bp (Utilities|Casting|CastToParkourGameModeBP (Game|GetGameMode)))
        (bind _isactive (Default|IsColorActive _asparkour_game_mode_bp "NewEnumerator0"))
        (if _isactive
          (Variables|Default|SetStopChecking1 true)
          ;[0.1562 0.1562 0.1562] Cambio de material
          (Rendering|Material|SetMaterial (Variables|Debug|GetStaticMeshComponent) 0 (Variables|Default|GetMatToSet1)))))
    (:then_1
      ;[0.07227 0.1302 0.07475] Comprobacion periodica
      (if (not (Variables|Default|GetStopChecking2))
        (bind _asparkour_game_mode_bp_2 (Utilities|Casting|CastToParkourGameModeBP (Game|GetGameMode)))
        (bind _isactive_2 (Default|IsColorActive _asparkour_game_mode_bp_2 "NewEnumerator3"))
        (if _isactive_2
          (Variables|Default|SetStopChecking2 true)
          ;[0.1562 0.1562 0.1562] Cambio de material
          (Rendering|Material|SetMaterial (Variables|Debug|GetStaticMeshComponent) 2 (Variables|Default|GetMatToSet2)))))))

(fn ConstructionScript)