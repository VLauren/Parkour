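; Building actor (Edificio02) that changes its look and turns solid once a specific color is active in the parkour game mode.
; Each Tick it polls ParkourGameModeBP for that color's state.
; When active, it swaps three material slots on its static mesh, enables actor collision and sets a flag that stops further checks, so the change is one-way.
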(event EventBeginPlay)

(event Collision|EventActorBeginOverlap
  (params (OtherActor :type Actor%20Object%20Reference)))

(event EventTick
  (params (DeltaSeconds :type Float%20%28single-precision%29))
  ;[0.07227 0.1302 0.07475] Comprobacion periodica
  (if (not (Variables|Default|GetStopChecking1))
    (bind _asparkour_game_mode_bp (Utilities|Casting|CastToParkourGameModeBP (Game|GetGameMode)))
    (bind _isactive (Default|IsColorActive _asparkour_game_mode_bp "NewEnumerator3"))
    (if _isactive
      (Variables|Default|SetStopChecking1 true)
      (Rendering|Material|SetMaterial (Variables|Debug|GetStaticMeshComponent) 0 (Variables|Default|GetMatToSet1))
      (Rendering|Material|SetMaterial (Variables|Debug|GetStaticMeshComponent) 1 (Variables|Default|GetMatToSet2))
      (Rendering|Material|SetMaterial (Variables|Debug|GetStaticMeshComponent) 2 (Variables|Default|GetMatToSet3))
      (Collision|SetActorEnableCollision true))))

(fn ConstructionScript)