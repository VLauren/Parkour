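; Player character with parkour movement: camera-relative walking and looking, a limited launch jump, automatic ledge climbing and wall running.
; Two border detectors track overlaps; when only B has one, a timeline lerps the actor up and forward.
; Touching a "RunWall" while falling with Space held zeroes gravity, locks height via plane constraint, pushes forward and aligns rotation to the wall.
; A DoN counter gates jumps, resetting on landing or wall contact.
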(event OnComponentBeginOverlap(WallDetect)
  (params (OverlappedComponent :type Primitive%20Component%20Object%20Reference) (OtherActor :type Actor%20Object%20Reference) (OtherComp :type Primitive%20Component%20Object%20Reference) (OtherBodyIndex :type Integer) (bFromSweep :type Boolean) (SweepResult :type Hit%20Result%20Structure%20%28by%20ref%29))
  (bind _returnvalue (Transformation|GetActorForwardVector))
  (bind _charactermovement (Variables|Character|GetCharacterMovement))
  (bind _charactermovement_2 (Variables|Character|GetCharacterMovement))
  (bind _charactermovement_3 (Variables|Character|GetCharacterMovement))
  (bind (_x _y) (Math|Vector|BreakVector _returnvalue))
  (bind _velocity (Variables|/Script/Engine.MovementComponent|GetVelocity _charactermovement))
  (bind (_x_2 _y_2) (Math|Vector|BreakVector _velocity))
  (Variables|Default|SetWallCollider OtherComp)
  (Variables|Default|SetDotResult 0.0)
  (Utilities|FlowControl|Sequence
    (:then_0
      ;[1 1 1] Salto
      (Utilities|FlowControl|DoN 1) ; enters at Reset
    )
    (:then_1
      (Variables|Default|SetPlayerDirection (Transformation|GetActorForwardVector (Components|GetOwner)))
      (if (and (Actor|ActorHasTag OtherActor "RunWall") (AI|Components|NavMovement|IsFalling (Variables|Character|GetCharacterMovement)))
        (Variables|Default|SetOnWall true)
        (Timeline|WallRun Play
          (:Update
            (if (> (Class|PlayerController|GetInputKeyTimeDown (Game|GetPlayerController 0) "SpaceBar") 0.0)
              (if (Variables|Default|GetOnWall)
                ;[0.6159 0.6837 1] Inicio/Mantengo WallRun
                (Variables|/Script/Engine.CharacterMovementComponent|SetGravityScale _charactermovement_3 0.0)
                (Class|MovementComponent|SetPlaneConstraintNormal _charactermovement_3 "0, 0,1.000000")
                (Physics|AddForce _charactermovement_3 (* (Variables|Default|GetPlayerDirection) 2e+04))
                (Transformation|SetActorRotation (Math|Conversions|RotationFromXVector (Math|Vector|RotateVector (- (Transformation|GetActorLocation) (.OutPointOnBody (Collision|GetClosestPointonCollision (Variables|Default|GetWallCollider) (Transformation|GetActorLocation) "None"))) "0.000000,-90.000000, 0")))
                (Transformation|SetActorRotation (Math|Conversions|RotationFromXVector (Math|Vector|RotateVector (Transformation|GetActorForwardVector) (Math|Rotator|MakeRotator 0.0 0.0 (- (Class|KismetMathLibrary|DegAtan2 _x_2 _y_2) (Class|KismetMathLibrary|DegAtan2 _x _y))))))
                (else
                  ;[0.2417 0.3217 0.5781] Cortar WallRun
                  (Variables|/Script/Engine.CharacterMovementComponent|SetGravityScale _charactermovement_2 1.0 :!label _label)
                  (Class|MovementComponent|SetPlaneConstraintNormal _charactermovement_2 "0, 0, 0")
                  (Variables|Default|SetOnWall false)))
              (else
                (goto _label)))))))))

(event OnComponentEndOverlap(WallDetect)
  (params (OverlappedComponent :type Primitive%20Component%20Object%20Reference) (OtherActor :type Actor%20Object%20Reference) (OtherComp :type Primitive%20Component%20Object%20Reference) (OtherBodyIndex :type Integer))
  (bind _returnvalue (Transformation|GetActorForwardVector))
  (bind _charactermovement (Variables|Character|GetCharacterMovement))
  (bind _charactermovement_2 (Variables|Character|GetCharacterMovement))
  (bind _charactermovement_3 (Variables|Character|GetCharacterMovement))
  (bind (_x _y) (Math|Vector|BreakVector _returnvalue))
  (bind _velocity (Variables|/Script/Engine.MovementComponent|GetVelocity _charactermovement))
  (bind (_x_2 _y_2) (Math|Vector|BreakVector _velocity))
  (Utilities|FlowControl|Sequence
    (:then_0
      (Timeline|WallRun Stop
        (:Update
          (if (> (Class|PlayerController|GetInputKeyTimeDown (Game|GetPlayerController 0) "SpaceBar") 0.0)
            (if (Variables|Default|GetOnWall)
              ;[0.6159 0.6837 1] Inicio/Mantengo WallRun
              (Variables|/Script/Engine.CharacterMovementComponent|SetGravityScale _charactermovement_3 0.0)
              (Class|MovementComponent|SetPlaneConstraintNormal _charactermovement_3 "0, 0,1.000000")
              (Physics|AddForce _charactermovement_3 (* (Variables|Default|GetPlayerDirection) 2e+04))
              (Transformation|SetActorRotation (Math|Conversions|RotationFromXVector (Math|Vector|RotateVector (- (Transformation|GetActorLocation) (.OutPointOnBody (Collision|GetClosestPointonCollision (Variables|Default|GetWallCollider) (Transformation|GetActorLocation) "None"))) "0.000000,-90.000000, 0")))
              (Transformation|SetActorRotation (Math|Conversions|RotationFromXVector (Math|Vector|RotateVector (Transformation|GetActorForwardVector) (Math|Rotator|MakeRotator 0.0 0.0 (- (Class|KismetMathLibrary|DegAtan2 _x_2 _y_2) (Class|KismetMathLibrary|DegAtan2 _x _y))))))
              (else
                ;[0.2417 0.3217 0.5781] Cortar WallRun
                (Variables|/Script/Engine.CharacterMovementComponent|SetGravityScale _charactermovement_2 1.0 :!label _label)
                (Class|MovementComponent|SetPlaneConstraintNormal _charactermovement_2 "0, 0, 0")
                (Variables|Default|SetOnWall false)))
            (else
              (goto _label))))))
    (:then_1
      (if (Actor|ActorHasTag OtherActor "RunWall")
        (goto _label)))))

(event OnComponentBeginOverlap(BorderDetectA)
  (params (OverlappedComponent :type Primitive%20Component%20Object%20Reference) (OtherActor :type Actor%20Object%20Reference) (OtherComp :type Primitive%20Component%20Object%20Reference) (OtherBodyIndex :type Integer) (bFromSweep :type Boolean) (SweepResult :type Hit%20Result%20Structure%20%28by%20ref%29))
  (Utilities|Array|Add (Variables|Default|GetAOverlaps) OverlappedComponent))

(event OnComponentBeginOverlap(BorderDetectB)
  (params (OverlappedComponent :type Primitive%20Component%20Object%20Reference) (OtherActor :type Actor%20Object%20Reference) (OtherComp :type Primitive%20Component%20Object%20Reference) (OtherBodyIndex :type Integer) (bFromSweep :type Boolean) (SweepResult :type Hit%20Result%20Structure%20%28by%20ref%29))
  (Utilities|Array|Add (Variables|Default|GetBOverlaps) OverlappedComponent))

(event OnComponentEndOverlap(BorderDetectB)
  (params (OverlappedComponent :type Primitive%20Component%20Object%20Reference) (OtherActor :type Actor%20Object%20Reference) (OtherComp :type Primitive%20Component%20Object%20Reference) (OtherBodyIndex :type Integer))
  (Utilities|Array|RemoveItem (Variables|Default|GetBOverlaps) OverlappedComponent))

(event OnComponentEndOverlap(BorderDetectA)
  (params (OverlappedComponent :type Primitive%20Component%20Object%20Reference) (OtherActor :type Actor%20Object%20Reference) (OtherComp :type Primitive%20Component%20Object%20Reference) (OtherBodyIndex :type Integer))
  (Utilities|Array|RemoveItem (Variables|Default|GetAOverlaps) OverlappedComponent))

(event EventBeginPlay
  (Class|MovementComponent|SetPlaneConstraintEnabled (Variables|Character|GetCharacterMovement) true)
  (Utilities|FlowControl|Delay 0.1)
  (Utilities|Array|Clear (Variables|Default|GetAOverlaps))
  (Utilities|Array|Clear (Variables|Default|GetBOverlaps)))

(event EventTick
  (params (DeltaSeconds :type Float%20%28single-precision%29))
  (bind _returnvalue (Transformation|GetActorLocation))
  (if (Math|Boolean|ANDBoolean (== (Utilities|Array|Length (Variables|Default|GetAOverlaps)) 0) (== (Utilities|Array|Length (Variables|Default|GetBOverlaps)) 1) (not (Variables|Default|GetClimbing)))
    (Variables|Default|SetClimbing true)
    ;[0.2473 0.3235 0.5521] Subir borde
    (Variables|Default|SetClimbStartPosition _returnvalue)
    (Variables|Default|SetClimbTargetPosition (+ _returnvalue (* (Transformation|GetActorForwardVector) 5e+01) (* (Transformation|GetActorUpVector) 8e+01)))
    (bind _time (Timeline|Climb PlayFromStart)
      (:Update
        (Transformation|SetActorLocation (Math|Vector|Lerp(Vector) (Variables|Default|GetClimbStartPosition) (Variables|Default|GetClimbTargetPosition) _time) false false))
      (:Finished
        (Variables|Default|SetClimbing false)))))

(event EventOnLanded
  (params (Hit :type Hit%20Result%20Structure%20%28by%20ref%29))
  ;[1 1 1] Salto
  (Utilities|FlowControl|DoN 1) ; enters at Reset
)

(event Input|ActionEvents|InputActionJump
  (params (Key :type Key%20Structure :default "None"))
  ;[1 1 1] Salto
  (:Pressed
    (bind _counter (Utilities|FlowControl|DoN 1)
      (:Exit
        (switch int _counter
          (:1
            (Character|LaunchCharacter "0, 0,420.000000" false true))))))
  (:Released
    (Character|StopJumping)))

(event Input|AxisEvents|InputAxisMoveRight
  (params (AxisValue :type Float%20%28single-precision%29))
  ;[0.1729 1 0.3234] Movimiento y camara
  (Pawn|Input|AddMovementInput (Math|Vector|GetRightVector (Math|Rotator|MakeRotator 0.0 0.0 (.Yaw (Math|Rotator|BreakRotator (Pawn|GetControlRotation :!class /Script/Engine.Pawn))))) AxisValue false))

(event Input|AxisEvents|InputAxisMoveForward
  (params (AxisValue :type Float%20%28single-precision%29))
  ;[0.1729 1 0.3234] Movimiento y camara
  (Pawn|Input|AddMovementInput (Math|Vector|GetForwardVector (Math|Rotator|MakeRotator 0.0 0.0 (.Yaw (Math|Rotator|BreakRotator (Pawn|GetControlRotation :!class /Script/Engine.Pawn))))) AxisValue false))

(event Input|AxisEvents|InputAxisLookRight
  (params (AxisValue :type Float%20%28single-precision%29))
  ;[0.1729 1 0.3234] Movimiento y camara
  (Pawn|Input|AddControllerYawInput AxisValue))

(event Input|AxisEvents|InputAxisLookUp
  (params (AxisValue :type Float%20%28single-precision%29))
  ;[0.1729 1 0.3234] Movimiento y camara
  (Pawn|Input|AddControllerPitchInput AxisValue))

(fn ConstructionScript)

(fn IsWallRunning
  (return (Variables|Default|GetOnWall)))

(fn IsMoving
  (return (> (Math|Vector|VectorLength (Variables|/Script/Engine.MovementComponent|GetVelocity (Variables|Character|GetCharacterMovement))) 0.0)))